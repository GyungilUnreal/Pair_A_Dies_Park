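; Debug player controller for split-screen play, adding input mapping and, outside DebugMode, spawning a second local player from controller 0.
; Input drives player 1's character, with player 0 fallback for GAS ability presses and gaze interaction.
; DebugMode adds parallel handlers targeting the controlled pawn and a Tab-toggled WBP_Debug widget.
; Mutually exclusive toggles provide ghost mode via a possessed SpectatorPawn and collision-free flying; C fires a test montage ability.
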(event Custom|SwitchGhostMode
  (bind _returnvalue (Pawn|GetControlledPawn))
  (if (not (Variables|Default|GetFlying))
    (if (Variables|Default|GetGhost)
      (Variables|Default|SetGhost false)
      (Pawn|Possess (Variables|Default|GetOriginalPawn))
      (Actor|DestroyActor (stale _returnvalue_2))
      (else
        (Variables|Default|SetGhost true)
        (Variables|Default|SetOriginalPawn _returnvalue)
        (bind _returnvalue_2 (Game|SpawnActorfromClass "/Script/Engine.SpectatorPawn" (Transformation|GetActorTransform _returnvalue) "Undefined" "MultiplyWithRoot" 0 0))
        (Collision|SetActorEnableCollision _returnvalue_2 false)
        (Pawn|Possess _returnvalue_2)))))

(event Custom|SwitchFlyingMode
  (if (not (Variables|Default|GetGhost))
    (if (Variables|Default|GetFlying)
      (Variables|Default|SetFlying false)
      (bind _as캐릭터 (Utilities|Casting|CastToCharacter (Pawn|GetControlledPawn)))
      (Pawn|Components|CharacterMovement|SetMovementMode (Variables|/Script/Engine.Character|GetCharacterMovement _as캐릭터) "MOVE_Walking" 0)
      (Collision|SetCollisionEnabled (Variables|/Script/Engine.Character|GetCapsuleComponent _as캐릭터) "QueryAndPhysics")
      (else
        (Variables|Default|SetFlying true)
        (bind _as캐릭터_2 (Utilities|Casting|CastToCharacter (Pawn|GetControlledPawn)))
        (Pawn|Components|CharacterMovement|SetMovementMode (Variables|/Script/Engine.Character|GetCharacterMovement _as캐릭터_2) "MOVE_Flying" 0)
        (Collision|SetCollisionEnabled (Variables|/Script/Engine.Character|GetCapsuleComponent _as캐릭터_2) "NoCollision")))))

(event Custom|TriggerUI
  (if (Variables|Default|GetDebugUI)
    (Variables|Default|SetDebugUI false)
    (if (Pawn|IsLocalController)
      (Input|SetInputModeGameOnly self false)
      (Variables|Default|SetbShowMouseCursor false)
      (Widget|RemovefromParent (stale _returnvalue)))
    (else
      (Variables|Default|SetDebugUI true)
      (if (Pawn|IsLocalController)
        (Input|SetInputModeUIOnly self 0 "DoNotLock" false)
        (Variables|Default|SetbShowMouseCursor true)
        (bind _returnvalue (UserInterface|CreateWidget "/Game/Collaborators/LKH/Split/Debug/WBP_Debug.WBP_Debug_C"))
        (UserInterface|Viewport|AddtoPlayerScreen _returnvalue)))))

(event Input|EnhancedActionEvents|EnhancedInputActionIA_Fire
  (params (ActionValue :type Boolean) (ElapsedSeconds :type Float%20%28double-precision%29) (TriggeredSeconds :type Float%20%28double-precision%29) (InputAction :type Input%20Action%20Object%20Reference :default "/Game/ThirdPerson/Input/Actions/IA_Fire.IA_Fire"))
  (bind _returnvalue (Game|GetPlayerCharacter 1))
  (bind _returnvalue_2 (Game|GetPlayerCharacter 0))
  (bind _returnvalue_3 (Game|GetPlayerCharacter 1))
  (bind _returnvalue_4 (Game|GetPlayerCharacter 0))
  (bind _returnvalue_5 (Ability|GetAbilitySystemComponent _returnvalue_2))
  (bind _returnvalue_6 (Ability|GetAbilitySystemComponent _returnvalue_4))
  (:Started
    (Utilities|IsValid _returnvalue
      (:Is%20Valid
        (Class|AbilitySystemComponent|PressInputID (Ability|GetAbilitySystemComponent _returnvalue) 1002))
      (:Is%20Not%20Valid
        (Utilities|IsValid _returnvalue_5
          (:Is%20Valid
            (Class|AbilitySystemComponent|PressInputID _returnvalue_5 1002))))))
  (:Completed
    (Utilities|IsValid _returnvalue_3
      (:Is%20Valid
        (Class|AbilitySystemComponent|ReleaseInputID (Ability|GetAbilitySystemComponent _returnvalue_3) 1002))
      (:Is%20Not%20Valid
        (Utilities|IsValid _returnvalue_6
          (:Is%20Valid
            (Class|AbilitySystemComponent|ReleaseInputID _returnvalue_6 1002)))))))

(event Input|EnhancedActionEvents|EnhancedInputActionIA_Move
  (params (ActionValue :type Vector%202D%20Structure) (ElapsedSeconds :type Float%20%28double-precision%29) (TriggeredSeconds :type Float%20%28double-precision%29) (InputAction :type Input%20Action%20Object%20Reference :default "/Game/ThirdPerson/Input/Actions/IA_Move.IA_Move"))
  (bind _returnvalue (Game|GetPlayerController 1))
  (bind _returnvalue_2 (Game|GetPlayerCharacter 1))
  (bind (_x _y) (Math|Vector2D|BreakVector2D ActionValue))
  (bind _returnvalue_3 (Pawn|GetControlRotation _returnvalue :!class /Script/Engine.Controller))
  (bind _yaw (Math|Rotator|BreakRotator _returnvalue_3))
  (bind _returnvalue_4 (Math|Rotator|MakeRotator 0.0 0.0 _yaw))
  (Utilities|IsValid _returnvalue_2
    (:Is%20Valid
      (Utilities|IsValid _returnvalue
        (:Is%20Valid
          (Pawn|Input|AddMovementInput _returnvalue_2 (Math|Vector|GetForwardVector _returnvalue_4) _y false)
          (Pawn|Input|AddMovementInput _returnvalue_2 (Math|Vector|GetRightVector _returnvalue_4) _x false))))))

(event Input|EnhancedActionEvents|EnhancedInputActionIA_Look
  (params (ActionValue :type Vector%202D%20Structure) (ElapsedSeconds :type Float%20%28double-precision%29) (TriggeredSeconds :type Float%20%28double-precision%29) (InputAction :type Input%20Action%20Object%20Reference :default "/Game/ThirdPerson/Input/Actions/IA_Look.IA_Look"))
  (bind (_x _y) (Math|Vector2D|BreakVector2D ActionValue))
  (bind _returnvalue (Game|GetPlayerCharacter 1))
  (Utilities|IsValid _returnvalue
    (:Is%20Valid
      (Pawn|Input|AddControllerYawInput _returnvalue _x)
      (Pawn|Input|AddControllerPitchInput _returnvalue _y))))

(event Input|EnhancedActionEvents|EnhancedInputActionIA_Jump
  (params (ActionValue :type Boolean) (ElapsedSeconds :type Float%20%28double-precision%29) (TriggeredSeconds :type Float%20%28double-precision%29) (InputAction :type Input%20Action%20Object%20Reference :default "/Game/ThirdPerson/Input/Actions/IA_Jump.IA_Jump"))
  (bind _returnvalue (Game|GetPlayerCharacter 1))
  (:Started
    (Utilities|IsValid _returnvalue
      (:Is%20Valid
        (Character|Jump _returnvalue))))
  (:Completed
    (Utilities|IsValid _returnvalue
      (:Is%20Valid
        (Character|StopJumping _returnvalue)))))

(event Input|EnhancedActionEvents|EnhancedInputActionIA_Jump
  (params (ActionValue :type Boolean) (ElapsedSeconds :type Float%20%28double-precision%29) (TriggeredSeconds :type Float%20%28double-precision%29) (InputAction :type Input%20Action%20Object%20Reference :default "/Game/ThirdPerson/Input/Actions/IA_Jump.IA_Jump"))
  (bind _returnvalue (Game|GetPlayerCharacter 1))
  (bind _returnvalue_2 (Game|GetPlayerCharacter 0))
  (bind _returnvalue_3 (Ability|GetAbilitySystemComponent _returnvalue_2))
  (:Started
    (Utilities|IsValid _returnvalue
      (:Is%20Valid
        (Class|AbilitySystemComponent|PressInputID (Ability|GetAbilitySystemComponent _returnvalue) 1001))
      (:Is%20Not%20Valid
        (Utilities|IsValid _returnvalue_3
          (:Is%20Valid
            (Class|AbilitySystemComponent|PressInputID _returnvalue_3 1001)))))))

(event Input|EnhancedActionEvents|EnhancedInputActionIA_UpDown
  (params (ActionValue :type Vector%202D%20Structure) (ElapsedSeconds :type Float%20%28double-precision%29) (TriggeredSeconds :type Float%20%28double-precision%29) (InputAction :type Input%20Action%20Object%20Reference :default "/Game/ThirdPerson/Input/Actions/IA_UpDown.IA_UpDown"))
  (bind (_x _y) (Math|Vector2D|BreakVector2D ActionValue))
  (bind _returnvalue (Pawn|GetControlledPawn))
  (bind _returnvalue_2 (Transformation|GetActorUpVector _returnvalue))
  (if (Variables|Default|GetFlying)
    (Pawn|Input|AddMovementInput _returnvalue _returnvalue_2 _x false)
    (Pawn|Input|AddMovementInput _returnvalue _returnvalue_2 _y false)))

(event Input|EnhancedActionEvents|EnhancedInputActionIA_Fire
  (params (ActionValue :type Boolean) (ElapsedSeconds :type Float%20%28double-precision%29) (TriggeredSeconds :type Float%20%28double-precision%29) (InputAction :type Input%20Action%20Object%20Reference :default "/Game/ThirdPerson/Input/Actions/IA_Fire.IA_Fire"))
  (bind _returnvalue (Pawn|GetControlledPawn))
  (bind _returnvalue_2 (Pawn|GetControlledPawn))
  (bind _returnvalue_3 (Ability|GetAbilitySystemComponent _returnvalue))
  (bind _returnvalue_4 (Ability|GetAbilitySystemComponent _returnvalue_2))
  (:Started
    (if (Variables|Default|GetDebugMode)
      (Utilities|IsValid _returnvalue_3
        (:Is%20Valid
          (Class|AbilitySystemComponent|PressInputID _returnvalue_3 1002)))))
  (:Completed
    (if (Variables|Default|GetDebugMode)
      (Utilities|IsValid _returnvalue_4
        (:Is%20Valid
          (Class|AbilitySystemComponent|ReleaseInputID _returnvalue_4 1002))))))

(event Input|EnhancedActionEvents|EnhancedInputActionIA_Jump
  (params (ActionValue :type Boolean) (ElapsedSeconds :type Float%20%28double-precision%29) (TriggeredSeconds :type Float%20%28double-precision%29) (InputAction :type Input%20Action%20Object%20Reference :default "/Game/ThirdPerson/Input/Actions/IA_Jump.IA_Jump"))
  (bind _returnvalue (Pawn|GetControlledPawn))
  (bind _returnvalue_2 (Ability|GetAbilitySystemComponent _returnvalue))
  (:Started
    (if (Variables|Default|GetDebugMode)
      (Utilities|IsValid _returnvalue_2
        (:Is%20Valid
          (Class|AbilitySystemComponent|PressInputID _returnvalue_2 1001))))))

(event EventBeginPlay
  (if (Variables|Default|GetDebugMode)
    (if (Pawn|IsLocalPlayerController)
      (Input|AddMappingContext (PlayerController|LocalPlayerSubsystems|GetEnhancedInputLocalPlayerSubsystem self) "/Game/ThirdPerson/Input/IMC_Default.IMC_Default" 0 "(bIgnoreAllPressedKeysUntilRelease=True,bForceImmediately=False,bNotifyUserSettings=False)"))
    (elif (== (Class|GameplayStatics|GetPlayerControllerID self) 0)
      (Input|AddMappingContext (PlayerController|LocalPlayerSubsystems|GetEnhancedInputLocalPlayerSubsystem self) "/Game/ThirdPerson/Input/IMC_Default.IMC_Default" 0 "(bIgnoreAllPressedKeysUntilRelease=True,bForceImmediately=False,bNotifyUserSettings=False)")
      (if (not (>= (Class|GameplayStatics|GetNumLocalPlayerControllers) 2))
        (Class|GameplayStatics|CreatePlayer -1)))))

(event Input|MouseEvents|RightMouseButton
  (params (Key :type Key%20Structure :default "None"))
  (bind _returnvalue (Game|GetPlayerCharacter 1))
  (bind _returnvalue_2 (Game|GetPlayerCharacter 0))
  (bind _returnvalue_3 (Game|GetPlayerCharacter 1))
  (bind _returnvalue_4 (Game|GetPlayerCharacter 0))
  (bind _returnvalue_5 (Ability|GetAbilitySystemComponent _returnvalue_4))
  (bind _returnvalue_6 (Ability|GetAbilitySystemComponent _returnvalue))
  (bind _returnvalue_7 (Ability|GetAbilitySystemComponent _returnvalue_2))
  (:Pressed
    (Utilities|IsValid _returnvalue
      (:Is%20Valid
        (Class|AbilitySystemComponent|PressInputID _returnvalue_6 1003)
        (Class|AbilitySystemComponent|InputCancel _returnvalue_6))
      (:Is%20Not%20Valid
        (Utilities|IsValid _returnvalue_7
          (:Is%20Valid
            (Class|AbilitySystemComponent|PressInputID _returnvalue_7 1003)
            (Class|AbilitySystemComponent|InputCancel _returnvalue_7))))))
  (:Released
    (Utilities|IsValid _returnvalue_3
      (:Is%20Valid
        (Class|AbilitySystemComponent|ReleaseInputID (Ability|GetAbilitySystemComponent _returnvalue_3) 1003))
      (:Is%20Not%20Valid
        (Utilities|IsValid _returnvalue_5
          (:Is%20Valid
            (Class|AbilitySystemComponent|ReleaseInputID _returnvalue_5 1003)))))))

(event Input|KeyboardEvents|F
  (params (Key :type Key%20Structure :default "None"))
  (bind _returnvalue (Game|GetPlayerCharacter 1))
  (bind _returnvalue_2 (Game|GetPlayerCharacter 0))
  (:Pressed
    (Utilities|IsValid _returnvalue
      (:Is%20Valid
        (Class|GazeInteractorComponent|TryInteract (Actor|GetComponentbyClass _returnvalue "/Script/Pair_A_Dies_Park.GazeInteractorComponent") _returnvalue))
      (:Is%20Not%20Valid
        (Utilities|IsValid _returnvalue_2
          (:Is%20Valid
            (Class|GazeInteractorComponent|TryInteract (Actor|GetComponentbyClass _returnvalue_2 "/Script/Pair_A_Dies_Park.GazeInteractorComponent") _returnvalue_2)))))))

(event Input|MouseEvents|RightMouseButton
  (params (Key :type Key%20Structure :default "None"))
  (bind _returnvalue (Pawn|GetControlledPawn))
  (bind _returnvalue_2 (Pawn|GetControlledPawn))
  (bind _returnvalue_3 (Ability|GetAbilitySystemComponent _returnvalue))
  (bind _returnvalue_4 (Ability|GetAbilitySystemComponent _returnvalue_2))
  (:Pressed
    (if (Variables|Default|GetDebugMode)
      (Utilities|IsValid _returnvalue_3
        (:Is%20Valid
          (Class|AbilitySystemComponent|PressInputID _returnvalue_3 1003)
          (Class|AbilitySystemComponent|InputCancel _returnvalue_3)))))
  (:Released
    (if (Variables|Default|GetDebugMode)
      (Utilities|IsValid _returnvalue_4
        (:Is%20Valid
          (Class|AbilitySystemComponent|ReleaseInputID _returnvalue_4 1003))))))

(event Input|KeyboardEvents|C
  (params (Key :type Key%20Structure :default "None"))
  (:Pressed
    (Abilities|TryActivateAbilitybyClass (Ability|GetAbilitySystemComponent (Pawn|GetControlledPawn)) "/Game/Collaborators/LKH/Split/GAS/Test/GA_TestMontage.GA_TestMontage_C" true)))

(event Input|KeyboardEvents|F
  (params (Key :type Key%20Structure :default "None"))
  (bind _returnvalue (Pawn|GetControlledPawn))
  (:Pressed
    (if (Variables|Default|GetDebugMode)
      (Class|GazeInteractorComponent|TryInteract (Actor|GetComponentbyClass _returnvalue "/Script/Pair_A_Dies_Park.GazeInteractorComponent") _returnvalue))))

(event Input|KeyboardEvents|Tab
  (params (Key :type Key%20Structure :default "None"))
  (:Pressed
    (if (Variables|Default|GetDebugMode)
      (CallFunction|TriggerUI))))

(fn ConstructionScript)