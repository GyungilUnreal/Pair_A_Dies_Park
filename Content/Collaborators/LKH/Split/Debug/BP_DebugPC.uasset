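; Debug player controller that drives ability input on the controlled pawn and adds a noclip toggle.
; The Enhanced Input actions for fire and jump forward fixed input IDs to the pawn's Ability System Component when it is valid.
; The Y key stores the current pawn and possesses a newly spawned SpectatorPawn at its transform.
; Pressing Y again repossesses the original pawn without destroying the spectator.
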(event Input|EnhancedActionEvents|EnhancedInputActionIA_Fire
  (params (ActionValue :type Boolean) (ElapsedSeconds :type Float%20%28double-precision%29) (TriggeredSeconds :type Float%20%28double-precision%29) (InputAction :type Input%20Action%20Object%20Reference :default "/Game/ThirdPerson/Input/Actions/IA_Fire.IA_Fire"))
  (bind _returnvalue (Pawn|GetControlledPawn))
  (bind _returnvalue_2 (Ability|GetAbilitySystemComponent _returnvalue))
  (:Started
    (Utilities|IsValid _returnvalue_2
      (:Is%20Valid
        (Class|AbilitySystemComponent|PressInputID _returnvalue_2 1002)))))

(event Input|EnhancedActionEvents|EnhancedInputActionIA_Jump
  (params (ActionValue :type Boolean) (ElapsedSeconds :type Float%20%28double-precision%29) (TriggeredSeconds :type Float%20%28double-precision%29) (InputAction :type Input%20Action%20Object%20Reference :default "/Game/ThirdPerson/Input/Actions/IA_Jump.IA_Jump"))
  (bind _returnvalue (Pawn|GetControlledPawn))
  (bind _returnvalue_2 (Ability|GetAbilitySystemComponent _returnvalue))
  (:Started
    (Utilities|IsValid _returnvalue_2
      (:Is%20Valid
        (Class|AbilitySystemComponent|PressInputID _returnvalue_2 1001)))))

(event EventBeginPlay)

(event EventTick
  (params (DeltaSeconds :type Float%20%28single-precision%29)))

(event Input|KeyboardEvents|Y
  (params (Key :type Key%20Structure :default "None"))
  (bind _returnvalue (Pawn|GetControlledPawn))
  (:Pressed
    (if (Variables|Default|GetNoclip)
      (Variables|Default|SetNoclip false)
      (Pawn|Possess (Variables|Default|GetOriginalPawn))
      (else
        (Variables|Default|SetNoclip true)
        (Variables|Default|SetOriginalPawn _returnvalue)
        (bind _returnvalue_2 (Game|SpawnActorfromClass "/Script/Engine.SpectatorPawn" (Transformation|GetActorTransform _returnvalue) "Undefined" "MultiplyWithRoot" 0 0))
        (Pawn|Possess _returnvalue_2)))))

(fn ConstructionScript)