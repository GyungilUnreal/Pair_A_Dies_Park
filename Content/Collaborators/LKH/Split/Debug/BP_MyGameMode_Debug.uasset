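; Debug game mode that sets up a four-controller split-screen boss session, sorting joining players into local and remote pairs.
; Once all four join, it spawns split characters at two PlayerStarts for one local and one remote controller.
; The other two controllers mirror those players through view targets, then loading ends and the game state plays the boss intro.
; DebugMode skips this, giving each login its own character at the first start.
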(event Custom|SpawnQuinnAndPossess
  (params (PC :type Player%20Controller%20Object%20Reference))
  (bind _returnvalue (Game|SpawnActorfromClass "/Game/Collaborators/LKH/Split/BP_Split_Character.BP_Split_Character_C" (Transformation|GetActorTransform (Utilities|Array|Get(acopy) (Variables|Default|GetPlayerStarts) 1)) "Undefined" "MultiplyWithRoot" 0 0))
  (Pawn|Possess PC _returnvalue))

(event Custom|SpawnAndPossess
  (params (PC :type Player%20Controller%20Object%20Reference))
  (bind _returnvalue (Game|SpawnActorfromClass "/Game/Collaborators/LKH/Split/BP_Split_Character.BP_Split_Character_C" (Transformation|GetActorTransform (Utilities|Array|Get(acopy) (Variables|Default|GetPlayerStarts))) "Undefined" "MultiplyWithRoot" 0 0))
  (Pawn|Possess PC _returnvalue))

(event Custom|SetCharacter
  (Game|Player|SetViewTargetwithBlend (Variables|Default|GetCS_1) (Variables|Default|GetLS_1) 0.0 "VTBlend_Linear" 0.0 false)
  (Game|Player|SetViewTargetwithBlend (Variables|Default|GetLS_2) (Variables|Default|GetCS_2) 0.0 "VTBlend_Linear" 0.0 false))

(event EventBeginPlay
  (bind _outactors (Actor|GetAllActorsOfClass "/Script/Engine.PlayerStart"))
  (Variables|Default|SetPlayerStarts _outactors))

(event EventPostLogin
  (params (NewPlayer :type Player%20Controller%20Object%20Reference))
  (if (Variables|Default|GetDebugMode)
    (Utilities|FlowControl|Delay 1.0)
    (CallFunction|SpawnandPossess NewPlayer)
    (else
      (if (Pawn|IsLocalController NewPlayer)
        (Utilities|IsValid (Variables|Default|GetLS_1)
          (:Is%20Valid
            (Variables|Default|SetLS_2 NewPlayer))
          (:Is%20Not%20Valid
            (Variables|Default|SetLS_1 NewPlayer)))
        (else
          (Utilities|IsValid (Variables|Default|GetCS_1)
            (:Is%20Valid
              (Variables|Default|SetCS_2 NewPlayer))
            (:Is%20Not%20Valid
              (Variables|Default|SetCS_1 NewPlayer)))))
      (bind _result (Math|Integer|IncrementInt (Variables|Default|GetCCount))
        (:%20%20
          (if (== _result 4)
            (Utilities|FlowControl|Delay 1.0)
            (Game|Player|SetViewTargetwithBlend (Variables|Default|GetLS_2) (Variables|Default|GetCS_2) 0.0 "VTBlend_Linear" 0.0 false)
            (Game|Player|SetViewTargetwithBlend (Variables|Default|GetCS_1) (Variables|Default|GetLS_1) 0.0 "VTBlend_Linear" 0.0 false)
            (CallFunction|SpawnandPossess (Variables|Default|GetLS_1))
            (CallFunction|SpawnQuinnandPossess (Variables|Default|GetCS_2))
            (Utilities|FlowControl|Delay 2.0)
            (bind _asbp_my_player_controller_debug (Utilities|Casting|CastToBP_MyPlayerController_Debug (Variables|Default|GetLS_1)))
            (Default|EndLoading _asbp_my_player_controller_debug)
            (Utilities|FlowControl|Sequence
              (:then_0
                (bind _asbp_my_player_controller_debug_2 (Utilities|Casting|CastToBP_MyPlayerController_Debug (Variables|Default|GetCS_1)))
                (Default|EndLoading _asbp_my_player_controller_debug_2)
                (bind _asbp_boss_game_state (Utilities|Casting|CastToBP_BossGameState (Game|GetGameState)))
                (Default|PlayBossIntro _asbp_boss_game_state))
              (:then_1
                (bind _asbp_my_player_controller_debug_3 (Utilities|Casting|CastToBP_MyPlayerController_Debug (Variables|Default|GetCS_2)))
                (Default|EndLoading _asbp_my_player_controller_debug_3)
                (bind _asbp_boss_game_state_2 (Utilities|Casting|CastToBP_BossGameState (Game|GetGameState)))
                (Default|PlayBossIntro _asbp_boss_game_state_2)))))))))

(fn ConstructionScript)