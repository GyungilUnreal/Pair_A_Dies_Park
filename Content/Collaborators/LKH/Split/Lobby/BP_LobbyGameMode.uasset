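; Lobby game mode for a two-player session that registers host and guest and launches the start scene.
; PostLogin casts joiners to BP_LobbyPC, triggers host or guest UI, assigns delayed default nicknames, shares them, and refreshes the host's Steam avatar list.
; OnLoadingSuccess spawns BP_Split_Character by temporarily setting the default pawn class.
; Other events toggle Player1's ready flag and start the intro through BP_Sequencer and both controllers.
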(event Custom|Ready
  (bind _player_1 (Variables|Default|GetPlayer_1))
  (Variables|/Game/Collaborators/LKH/Split/Lobby/BP_LobbyPC.BP_LobbyPC_C|SetReady _player_1 (not (Variables|/Game/Collaborators/LKH/Split/Lobby/BP_LobbyPC.BP_LobbyPC_C|GetReady _player_1))))

(event Custom|OnLoadingSuccess
  (params (PC :type Player%20Controller%20Object%20Reference))
  (Variables|Default|SetDefaultPawnClass "/Game/Collaborators/LKH/Split/BP_Split_Character.BP_Split_Character_C")
  (Class|GameModeBase|RestartPlayer PC)
  (Variables|Default|SetDefaultPawnClass 0))

(event Custom|PlayStartScene
  (bind _returnvalue (Actor|GetActorOfClass "/Game/Collaborators/LKH/Split/Lobby/BP_Sequencer.BP_Sequencer_C"))
  (Default|PlaySequence _returnvalue)
  (CallFunction|PlayStartScene2))

(event Custom|PlayStartScene_2
  (Default|PlayStartScene (Variables|Default|GetPlayer_1))
  (Default|PlayStartScene (Variables|Default|GetPlayer_2)))

(event EventPostLogin
  (params (NewPlayer :type Player%20Controller%20Object%20Reference))
  (Utilities|IsValid (Variables|Default|GetPlayer_1)
    (:Is%20Valid
      (bind _asbp_lobby_pc (Utilities|Casting|CastToBP_LobbyPC NewPlayer))
      (bind _output_get (Variables|Default|SetPlayer_2 _asbp_lobby_pc))
      (Variables|/Game/Collaborators/LKH/Split/Lobby/BP_LobbyPC.BP_LobbyPC_C|SetGuestUITrigger _output_get true)
      (Utilities|FlowControl|Delay 1.0)
      (Variables|/Game/Collaborators/LKH/Split/Lobby/BP_LobbyPC.BP_LobbyPC_C|SetNickname _output_get "Player_2")
      (Utilities|FlowControl|Delay 1.0)
      (Variables|/Game/Collaborators/LKH/Split/Lobby/BP_LobbyPC.BP_LobbyPC_C|SetPlayer_1_Nickname _output_get (Variables|/Game/Collaborators/LKH/Split/Lobby/BP_LobbyPC.BP_LobbyPC_C|GetNickname (Variables|Default|GetPlayer_1)))
      (Variables|/Game/Collaborators/LKH/Split/Lobby/BP_LobbyPC.BP_LobbyPC_C|SetPlayer_2_Nickname (Variables|Default|GetPlayer_2) (Variables|/Game/Collaborators/LKH/Split/Lobby/BP_LobbyPC.BP_LobbyPC_C|GetNickname (Variables|Default|GetPlayer_2)))
      (Variables|/Game/Collaborators/LKH/Split/Lobby/BP_LobbyPC.BP_LobbyPC_C|SetPlayer_2_Nickname (Variables|Default|GetPlayer_1) (Variables|/Game/Collaborators/LKH/Split/Lobby/BP_LobbyPC.BP_LobbyPC_C|GetNickname (Variables|Default|GetPlayer_2)))
      (Class|SteamAvatarListWidget|BindandBuildList (Variables|/Game/Collaborators/LKH/Split/Lobby/BP_LobbyPC.BP_LobbyPC_C|GetSteamAvatarUI (Variables|Default|GetPlayer_1)) true))
    (:Is%20Not%20Valid
      (bind _asbp_lobby_pc_2 (Utilities|Casting|CastToBP_LobbyPC NewPlayer))
      (bind _output_get_2 (Variables|Default|SetPlayer_1 _asbp_lobby_pc_2))
      (Variables|/Game/Collaborators/LKH/Split/Lobby/BP_LobbyPC.BP_LobbyPC_C|SetHostUITrigger _output_get_2 true)
      (Utilities|FlowControl|Delay 1.0)
      (Variables|/Game/Collaborators/LKH/Split/Lobby/BP_LobbyPC.BP_LobbyPC_C|SetNickname _output_get_2 "Player_1")
      (Utilities|FlowControl|Delay 1.0)
      (Variables|/Game/Collaborators/LKH/Split/Lobby/BP_LobbyPC.BP_LobbyPC_C|SetPlayer_1_Nickname _output_get_2 (Variables|/Game/Collaborators/LKH/Split/Lobby/BP_LobbyPC.BP_LobbyPC_C|GetNickname (Variables|Default|GetPlayer_1))))))

(fn ConstructionScript)