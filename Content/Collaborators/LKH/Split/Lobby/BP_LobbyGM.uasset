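; BP_LobbyGM is the lobby game mode that registers two players and starts the match.
; PostLogin stores the joining BP_LobbyPC as Player1 or Player2, assigns a default nickname, then after a one-second delay copies nicknames between the controllers.
; GameStart ignores its controller inputs and opens ThirdPersonMap by name.
; An unconnected destroy, find and join LAN session chain for PC2 never runs.
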(event Custom|GameStart
  (params (PC_1 :type Player%20Controller%20Object%20Reference) (PC_2 :type Player%20Controller%20Object%20Reference))
  (Game|OpenLevel(byName) "ThirdPersonMap"))

(event EventBeginPlay)

(event EventTick
  (params (DeltaSeconds :type Float%20%28single-precision%29)))

(event EventPostLogin
  (params (NewPlayer :type Player%20Controller%20Object%20Reference))
  (Utilities|IsValid (Variables|Default|GetPlayer_1)
    (:Is%20Valid
      (bind _asbp_lobby_pc (Utilities|Casting|CastToBP_LobbyPC NewPlayer))
      (bind _output_get (Variables|Default|SetPlayer_2 _asbp_lobby_pc))
      (Variables|/Game/Split/Lobby/BP_LobbyPC.BP_LobbyPC_C|SetNickname _output_get "Player_2")
      (Utilities|FlowControl|Delay 1.0)
      (Variables|/Game/Split/Lobby/BP_LobbyPC.BP_LobbyPC_C|SetPlayer_1_Nickname _output_get (Variables|/Game/Split/Lobby/BP_LobbyPC.BP_LobbyPC_C|GetNickname (Variables|Default|GetPlayer_1)))
      (Variables|/Game/Split/Lobby/BP_LobbyPC.BP_LobbyPC_C|SetPlayer_2_Nickname (Variables|Default|GetPlayer_2) (Variables|/Game/Split/Lobby/BP_LobbyPC.BP_LobbyPC_C|GetNickname (Variables|Default|GetPlayer_2)))
      (Variables|/Game/Split/Lobby/BP_LobbyPC.BP_LobbyPC_C|SetPlayer_2_Nickname (Variables|Default|GetPlayer_1) (Variables|/Game/Split/Lobby/BP_LobbyPC.BP_LobbyPC_C|GetNickname (Variables|Default|GetPlayer_2))))
    (:Is%20Not%20Valid
      (bind _asbp_lobby_pc_2 (Utilities|Casting|CastToBP_LobbyPC NewPlayer))
      (bind _output_get_2 (Variables|Default|SetPlayer_1 _asbp_lobby_pc_2))
      (Variables|/Game/Split/Lobby/BP_LobbyPC.BP_LobbyPC_C|SetNickname _output_get_2 "Player_1")
      (Utilities|FlowControl|Delay 1.0)
      (Variables|/Game/Split/Lobby/BP_LobbyPC.BP_LobbyPC_C|SetPlayer_1_Nickname _output_get_2 (Variables|/Game/Split/Lobby/BP_LobbyPC.BP_LobbyPC_C|GetNickname (Variables|Default|GetPlayer_1))))))

(fn ConstructionScript)