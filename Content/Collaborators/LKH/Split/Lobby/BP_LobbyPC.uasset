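; Lobby player controller that shows host or guest UI, handles Enter for ready/start and Tab for options, and removes the second local player.
; RepNotify variables create the role's widget, update nicknames and enable the host's Start button.
; Ready, loading-success and start-scene events forward to BP_LobbyGameMode.
; StartScene's RepNotify switches to a cine camera, then timed events show a dark screen and later restore lobby UI and pawn view as failed-travel fallback.
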(event Custom|Ready_PC
  (bind _asbp_lobby_game_mode (Utilities|Casting|CastToBP_LobbyGameMode (Game|GetGameMode)))
  (Default|Ready _asbp_lobby_game_mode))

(event Custom|Resume
  (bind _guestui (Variables|Default|GetGuestUI))
  (bind _hostui (Variables|Default|GetHostUI))
  (if (Variables|Default|GetSettings)
    (Variables|Default|SetSettings false)
    (Widget|RemovefromParent (stale Input|KeyboardEvents|Tab _returnvalue))
    (Variables|Default|SetbShowMouseCursor false)
    (Input|SetInputModeGameOnly self false)
    (Utilities|IsValid _hostui
      (:Is%20Valid
        (Widget|SetVisibility _hostui "SelfHitTestInvisible"))
      (:Is%20Not%20Valid
        (Utilities|IsValid _guestui
          (:Is%20Valid
            (Widget|SetVisibility _guestui "SelfHitTestInvisible")))))))

(event Custom|OnLoadingSuccess
  (bind _asbp_lobby_game_mode (Utilities|Casting|CastToBP_LobbyGameMode (Game|GetGameMode)))
  (Default|OnLoadingSuccess _asbp_lobby_game_mode self))

(event Custom|PlayStartScene_RPC
  (bind _asbp_lobby_game_mode (Utilities|Casting|CastToBP_LobbyGameMode (Game|GetGameMode)))
  (Default|PlayStartScene _asbp_lobby_game_mode))

(event Custom|FailedTravel
  (Utilities|FlowControl|Delay 1e+01)
  (if (Variables|Default|GetHostUITrigger)
    (bind _returnvalue (UserInterface|CreateWidget "/Game/Collaborators/LKH/Split/Lobby/UI/WBP_Lobby_Host.WBP_Lobby_Host_C"))
    (bind _output_get (Variables|Default|SetHostUI _returnvalue))
    (UserInterface|Viewport|AddtoPlayerScreen _output_get)
    (else
      (bind _returnvalue_2 (UserInterface|CreateWidget "/Game/Collaborators/LKH/Split/Lobby/UI/WBP_Lobby_Guest.WBP_Lobby_Guest_C"))
      (bind _output_get_2 (Variables|Default|SetGuestUI _returnvalue_2))
      (UserInterface|Viewport|AddtoPlayerScreen _output_get_2)))
  (Widget|RemovefromParent (stale Custom|LoadingTravel _returnvalue))
  (Game|Player|SetViewTargetwithBlend (Pawn|GetControlledPawn) 0.0 "VTBlend_Linear" 0.0 false))

(event Custom|LoadingTravel
  (Utilities|FlowControl|Delay 5.0)
  (bind _returnvalue (UserInterface|CreateWidget "/Game/Collaborators/LKH/Split/Lobby/UI/WBP_Dark.WBP_Dark_C"))
  (UserInterface|Viewport|AddtoViewport _returnvalue 0))

(event EventBeginPlay
  (if (== (Class|GameplayStatics|GetPlayerControllerID self) 1)
    (Actor|DestroyActor (Pawn|GetControlledPawn))
    (Class|GameplayStatics|RemovePlayer self true)
    (elif (Pawn|IsLocalController)
      (bind _returnvalue (UserInterface|CreateWidget "/Game/Collaborators/LKH/Split/Lobby/UI/WBP_Loading.WBP_Loading_C"))
      (UserInterface|Viewport|AddtoPlayerScreen _returnvalue 1000)
      (Input|SetInputModeGameOnly self false)
      (Input|AddMappingContext (PlayerController|LocalPlayerSubsystems|GetEnhancedInputLocalPlayerSubsystem self) "/Game/ThirdPerson/Input/IMC_Default.IMC_Default" 0 "(bIgnoreAllPressedKeysUntilRelease=True,bForceImmediately=False,bNotifyUserSettings=False)"))))

(event EventUnPossess
  (params (UnpossessedPawn :type Pawn%20Object%20Reference))
  (Actor|DestroyActor UnpossessedPawn))

(event Input|KeyboardEvents|Enter
  (params (Key :type Key%20Structure :default "None"))
  (bind _hostui (Variables|Default|GetHostUI))
  (:Pressed
    (if (Variables|Default|GetGuestUITrigger)
      (Default|PressReady (Variables|Default|GetGuestUI))
      (elif (Variables|Default|GetHostUITrigger)
        (if (Class|Widget|GetIsEnabled (Variables|/Game/Collaborators/LKH/Split/Lobby/UI/WBP_Lobby_Host.WBP_Lobby_Host_C|GetStartButton _hostui))
          (Default|PressStart _hostui))))))

(event Input|KeyboardEvents|Tab
  (params (Key :type Key%20Structure :default "None"))
  (bind _guestui (Variables|Default|GetGuestUI))
  (bind _hostui (Variables|Default|GetHostUI))
  (bind _guestui_2 (Variables|Default|GetGuestUI))
  (bind _hostui_2 (Variables|Default|GetHostUI))
  (:Pressed
    (if (Variables|Default|GetSettings)
      (Variables|Default|SetSettings false)
      (Widget|RemovefromParent (stale _returnvalue))
      (Variables|Default|SetbShowMouseCursor false)
      (Input|SetInputModeGameOnly self false)
      (Utilities|IsValid _hostui
        (:Is%20Valid
          (Widget|SetVisibility _hostui "SelfHitTestInvisible"))
        (:Is%20Not%20Valid
          (Utilities|IsValid _guestui
            (:Is%20Valid
              (Widget|SetVisibility _guestui "SelfHitTestInvisible")))))
      (else
        (Variables|Default|SetSettings true)
        (bind _returnvalue (UserInterface|CreateWidget "/Game/Collaborators/LKH/Split/Lobby/UI/WBP_InGameOptions.WBP_InGameOptions_C"))
        (UserInterface|Viewport|AddtoPlayerScreen _returnvalue)
        (Variables|Default|SetbShowMouseCursor true)
        (Input|SetInputModeUIOnly self _returnvalue "DoNotLock" false)
        (Utilities|IsValid _hostui_2
          (:Is%20Valid
            (Widget|SetVisibility _hostui_2 "Collapsed"))
          (:Is%20Not%20Valid
            (Utilities|IsValid _guestui_2
              (:Is%20Valid
                (Widget|SetVisibility _guestui_2 "Collapsed")))))))))

(fn ConstructionScript)

(fn OnRepPlayer1Nickname
  (bind _hostui (Variables|Default|GetHostUI))
  (if (Pawn|IsLocalController)
    (Utilities|IsValid _hostui
      (:Is%20Valid
        (Variables|/Script/UMG.TextBlock|SetText (Variables|/Game/Collaborators/LKH/Split/Lobby/UI/WBP_Lobby_Host.WBP_Lobby_Host_C|GetPlayer_1_Nickname _hostui) (Variables|Default|GetPlayer_1_Nickname)))
      (:Is%20Not%20Valid
        (Variables|/Script/UMG.TextBlock|SetText (Variables|/Game/Collaborators/LKH/Split/Lobby/UI/WBP_Lobby_Guest.WBP_Lobby_Guest_C|GetPlayer_1_Nickname (Variables|Default|GetGuestUI)) (Variables|Default|GetPlayer_1_Nickname))))))

(fn OnRepPlayer2Nickname
  (bind _hostui (Variables|Default|GetHostUI))
  (if (Pawn|IsLocalController)
    (Utilities|IsValid _hostui
      (:Is%20Valid
        (Variables|/Script/UMG.TextBlock|SetText (Variables|/Game/Collaborators/LKH/Split/Lobby/UI/WBP_Lobby_Host.WBP_Lobby_Host_C|GetPlayer_2_Nickname _hostui) (Variables|Default|GetPlayer_2_Nickname))
        (Variables|/Script/UMG.TextBlock|SetText (Variables|/Game/Collaborators/LKH/Split/Lobby/UI/WBP_Lobby_Host.WBP_Lobby_Host_C|GetStart _hostui) "짐싸길 기다리는 중..."))
      (:Is%20Not%20Valid
        (Variables|/Script/UMG.TextBlock|SetText (Variables|/Game/Collaborators/LKH/Split/Lobby/UI/WBP_Lobby_Guest.WBP_Lobby_Guest_C|GetPlayer_2_Nickname (Variables|Default|GetGuestUI)) (Variables|Default|GetPlayer_2_Nickname))))))

(fn OnRepHostUITrigger
  (if (Pawn|IsLocalController)
    (bind _returnvalue (UserInterface|CreateWidget "/Game/Collaborators/LKH/Split/Lobby/UI/WBP_Lobby_Host.WBP_Lobby_Host_C"))
    (bind _output_get (Variables|Default|SetHostUI _returnvalue))
    (UserInterface|Viewport|AddtoPlayerScreen _output_get)))

(fn OnRepGuestUITrigger
  (if (Pawn|IsLocalController)
    (bind _returnvalue (UserInterface|CreateWidget "/Game/Collaborators/LKH/Split/Lobby/UI/WBP_Lobby_Guest.WBP_Lobby_Guest_C"))
    (bind _output_get (Variables|Default|SetGuestUI _returnvalue))
    (UserInterface|Viewport|AddtoPlayerScreen _output_get)))

(fn OnRepReady
  (bind _hostui (Variables|Default|GetHostUI))
  (Widget|SetIsEnabled (Variables|/Game/Collaborators/LKH/Split/Lobby/UI/WBP_Lobby_Host.WBP_Lobby_Host_C|GetStartButton _hostui) (Variables|Default|GetReady))
  (Variables|/Script/UMG.TextBlock|SetText (Variables|/Game/Collaborators/LKH/Split/Lobby/UI/WBP_Lobby_Host.WBP_Lobby_Host_C|GetStart _hostui) "[Enter]여정을 떠나기"))

(fn OnRepStartScene
  (bind _returnvalue (Actor|GetActorOfClass "/Script/CinematicCamera.CineCameraActor"))
  (Game|Player|SetViewTargetwithBlend _returnvalue 0.0 "VTBlend_Linear" 0.0 false)
  (Viewport|RemoveAllWidgets)
  (CallFunction|LoadingTravel)
  (CallFunction|FailedTravel))