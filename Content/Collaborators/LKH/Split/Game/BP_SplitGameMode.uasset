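; Game mode for a networked split-screen setup that mirrors one host player and one remote player across both machines.
; PostLogin sorts controllers into two local and two remote slots, and the fourth login starts setup after a short delay.
; The second local and first remote controllers become viewers targeting the opposite side's active controller.
; The first local and second remote controllers each possess a newly spawned third-person character at the same location.
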(event Custom|SpawnQuinnAndPossess
  (params (PC :type Player%20Controller%20Object%20Reference))
  (bind _returnvalue (Game|SpawnActorfromClass "/Game/ThirdPerson/Blueprints/BP_ThirdPersonCharacter.BP_ThirdPersonCharacter_C" (Math|Transform|MakeTransform "500.000000,500.000000,0.000000") "Undefined" "MultiplyWithRoot" 0 0))
  (Pawn|Possess PC _returnvalue))

(event Custom|SpawnAndPossess
  (params (PC :type Player%20Controller%20Object%20Reference))
  (bind _returnvalue (Game|SpawnActorfromClass "/Game/ThirdPerson/Blueprints/BP_ThirdPersonCharacter.BP_ThirdPersonCharacter_C" (Math|Transform|MakeTransform "500.000000,500.000000,0.000000") "Undefined" "MultiplyWithRoot" 0 0))
  (Pawn|Possess PC _returnvalue))

(event EventBeginPlay)

(event EventPostLogin
  (params (NewPlayer :type Player%20Controller%20Object%20Reference))
  (if (Pawn|IsLocalController NewPlayer)
    (Utilities|IsValid (Variables|Default|GetLS_1)
      (:Is%20Valid
        (Variables|Default|SetLS_2 NewPlayer))
      (:Is%20Not%20Valid
        (Variables|Default|SetLS_1 NewPlayer)))
    (else
      (Utilities|IsValid (Variables|Default|GetCS_1)
        (:Is%20Valid
          (Variables|Default|SetCS_2 NewPlayer))
        (:Is%20Not%20Valid
          (Variables|Default|SetCS_1 NewPlayer)))))
  (bind _result (Math|Integer|IncrementInt (Variables|Default|GetCCount))
    (:%20%20
      (if (== _result 4)
        (Utilities|FlowControl|Delay 1.0)
        (Game|Player|SetViewTargetwithBlend (Variables|Default|GetLS_2) (Variables|Default|GetCS_2) 0.0 "VTBlend_Linear" 0.0 false)
        (Game|Player|SetViewTargetwithBlend (Variables|Default|GetCS_1) (Variables|Default|GetLS_1) 0.0 "VTBlend_Linear" 0.0 false)
        (CallFunction|SpawnandPossess (Variables|Default|GetLS_1))
        (CallFunction|SpawnQuinnandPossess (Variables|Default|GetCS_2))))))

(fn ConstructionScript)