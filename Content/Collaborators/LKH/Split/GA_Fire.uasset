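; GA_Fire is a Gameplay Ability that launches the avatar Character along its forward vector, acting as an instant forward burst.
; ActivateAbility commits, applies a strong additive LaunchCharacter impulse and ends immediately.
; CommitExecute treats the source object as an ItemAbilityComponent and notifies it that the owning actor consumed the ability, tying use to the granting item.
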(event Ability|EventActivateAbility
  (Ability|CommitAbility)
  (bind _as캐릭터 (Utilities|Casting|CastToCharacter (Ability|GetAvatarActorfromActorInfo)))
  (Character|LaunchCharacter _as캐릭터 (* (Transformation|GetActorForwardVector _as캐릭터) 5e+03) false false)
  (Ability|EndAbility))

(event Ability|EventOnEndAbility
  (params (bWasCancelled :type Boolean)))

(event Ability|EventCommitExecute
  (bind _asitem_ability_component (Utilities|Casting|CastToItemAbilityComponent (Ability|GetCurrentSourceObject)))
  (Class|ItemAbilityComponent|NotifyAbilityConsumed _asitem_ability_component (Ability|GetOwningActorfromActorInfo)))