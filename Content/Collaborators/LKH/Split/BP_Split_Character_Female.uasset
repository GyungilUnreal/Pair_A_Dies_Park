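; Player character Blueprint for the female character in a split setup, wiring test abilities and debug input to its components.
; On BeginPlay it grants two test Gameplay Abilities (GA_TestMontage, GA_Test2) through its Ability System Component.
; E triggers GazeInteractor interaction, while SpaceBar and C drive the PlayerFall component's mash input and let-go action.
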(event EventBeginPlay
  (bind _abilitysystemcomp (Variables|Default|GetAbilitySystemComp))
  (GameplayAbilities|GiveAbility _abilitysystemcomp "/Game/Collaborators/LKH/Split/GAS/Test/GA_TestMontage.GA_TestMontage_C" 0 -1)
  (GameplayAbilities|GiveAbility _abilitysystemcomp "/Game/Collaborators/LKH/Split/GAS/Test/GA_Test2.GA_Test2_C" 0 -1))

(event Collision|EventActorBeginOverlap
  (params (OtherActor :type Actor%20Object%20Reference)))

(event EventTick
  (params (DeltaSeconds :type Float%20%28single-precision%29)))

(event Input|KeyboardEvents|E
  (params (Key :type Key%20Structure :default "None"))
  (:Pressed
    (Class|GazeInteractorComponent|TryInteract (Variables|Default|GetGazeInteractor) self)))

(event Input|KeyboardEvents|C
  (params (Key :type Key%20Structure :default "None"))
  (:Pressed
    (Class|PlayerFallComponent|LetGo (Variables|Default|GetPlayerFall))))

(event Input|KeyboardEvents|SpaceBar
  (params (Key :type Key%20Structure :default "None"))
  (:Pressed
    (Class|PlayerFallComponent|InputMashF (Variables|Default|GetPlayerFall))))

(fn ConstructionScript)