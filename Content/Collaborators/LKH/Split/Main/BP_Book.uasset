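; BP_Book is a book actor built from many page components that animates a block of pages turning over.
; On Tick it advances an alpha by frame time times a Speed variable until it passes one.
; That alpha drives a rotator lerp that swings nine of the middle-numbered pages together through a half turn.
; The many other page components are referenced in the graph but left unconnected, and BeginPlay and the construction script are empty.
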(event EventBeginPlay)

(event EventTick
  (params (DeltaSeconds :type Float%20%28single-precision%29))
  (if (<= (Variables|Default|GetDelta) 1.0)
    (bind _output_get (Variables|Default|SetDelta (+ (Variables|Default|GetDelta) (* DeltaSeconds (Variables|Default|GetSpeed)))))
    (Transformation|SetRelativeRotation (Variables|Default|GetPage_019) (Math|Rotator|Lerp(Rotator) "-90.000000,0.000000,0.000000" "90.000000,0.000000,0.000000" _output_get) false false)))

(fn ConstructionScript)