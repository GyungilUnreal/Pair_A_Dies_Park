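; BP_MainGM, apparently the main game mode, handles two-player LAN session hosting, searching and joining through custom events.
; Creating a session opens the Lobby level as a listen server on success.
; Searching hands up to five results to the calling UI to refresh its list, for joining a given session.
; A quick-join event searches and joins the first result without checking for an empty list; failures are unhandled.
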(event Custom|FindAndJoinSession
  (params (PC :type Player%20Controller%20Object%20Reference))
  (bind _results (|FindSessions PC 5 true)
    (:OnSuccess
      (|JoinSession PC (Utilities|Array|Get(acopy) _results)))))

(event Custom|FindSession
  (params (PC :type Player%20Controller%20Object%20Reference) (UI :type WBP%20Main%202%20Object%20Reference))
  (bind _results (|FindSessions PC 5 true)
    (:OnSuccess
      (Variables|/Game/Collaborators/LKH/Split/Main/UI/WBP_Main_2.WBP_Main_2_C|SetSessionList UI _results)
      (Default|RefreshSessionList UI))))

(event Custom|CreateSession
  (params (PC :type Player%20Controller%20Object%20Reference))
  (|Session PC 2 true
    (:OnSuccess
      (Game|OpenLevel(byName) "Lobby?listen" false))))

(event Custom|JoinSession
  (params (PC :type Player%20Controller%20Object%20Reference) (Session :type Blueprint%20Session%20Result%20Structure))
  (|JoinSession PC Session))

(event EventBeginPlay)

(event EventTick
  (params (DeltaSeconds :type Float%20%28single-precision%29)))

(fn ConstructionScript)