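; BP_Bookmark is a bookmark actor that slides vertically in and out of view in front of the scene's CineCamera.
; BeginPlay caches the camera component; BookmarkAppears and BookmarkDisappears play or reverse one shared timeline that lerps the actor's position.
; The same alpha drives manual focus distance toward the bookmark, applied only from the halfway point when appearing but throughout when disappearing, selected by the Reverse flag.
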(event Custom|BookmarkAppears
  (bind _camera (Variables|Default|GetCamera))
  (Variables|Default|SetbReverse false)
  (bind _새_트랙_0 (Timeline|타임라인 Play)
    (:Update
      (if (Variables|Default|GetbReverse)
        (Transformation|SetActorTransform (Math|Transform|MakeTransform (Math|Vector|Lerp(Vector) "80.000000,0.000000,-10.000000" "80.000000,0.000000,17.000000" _새_트랙_0) "20.000000,180.000000,0.000000" "0.066000,0.066000,0.066000"))
        (Variables|/Script/CinematicCamera.CineCameraComponent|SetFocusSettings _camera (Utilities|Struct|MakeCameraFocusSettings "Manual" (Math|Float|Lerp 1.5e+02 8e+01 _새_트랙_0)))
        (else
          (Transformation|SetActorTransform (Math|Transform|MakeTransform (Math|Vector|Lerp(Vector) "80.000000,0.000000,-10.000000" "80.000000,0.000000,17.000000" _새_트랙_0) "20.000000,180.000000,0.000000" "0.066000,0.066000,0.066000"))
          (if (>= _새_트랙_0 0.5)
            (Variables|/Script/CinematicCamera.CineCameraComponent|SetFocusSettings _camera (Utilities|Struct|MakeCameraFocusSettings "Manual" (Math|Float|Lerp 1.5e+02 8e+01 _새_트랙_0)))))))))

(event Custom|BookmarkDisappears
  (bind _camera (Variables|Default|GetCamera))
  (Variables|Default|SetbReverse true)
  (bind _새_트랙_0 (Timeline|타임라인 Reverse)
    (:Update
      (if (Variables|Default|GetbReverse)
        (Transformation|SetActorTransform (Math|Transform|MakeTransform (Math|Vector|Lerp(Vector) "80.000000,0.000000,-10.000000" "80.000000,0.000000,17.000000" _새_트랙_0) "20.000000,180.000000,0.000000" "0.066000,0.066000,0.066000"))
        (Variables|/Script/CinematicCamera.CineCameraComponent|SetFocusSettings _camera (Utilities|Struct|MakeCameraFocusSettings "Manual" (Math|Float|Lerp 1.5e+02 8e+01 _새_트랙_0)))
        (else
          (Transformation|SetActorTransform (Math|Transform|MakeTransform (Math|Vector|Lerp(Vector) "80.000000,0.000000,-10.000000" "80.000000,0.000000,17.000000" _새_트랙_0) "20.000000,180.000000,0.000000" "0.066000,0.066000,0.066000"))
          (if (>= _새_트랙_0 0.5)
            (Variables|/Script/CinematicCamera.CineCameraComponent|SetFocusSettings _camera (Utilities|Struct|MakeCameraFocusSettings "Manual" (Math|Float|Lerp 1.5e+02 8e+01 _새_트랙_0)))))))))

(event EventBeginPlay
  (bind _returnvalue (Actor|GetActorOfClass "/Script/CinematicCamera.CineCameraActor"))
  (Variables|Default|SetCamera (Class|CineCameraActor|GetCineCameraComponent _returnvalue)))

(event Collision|EventActorBeginOverlap
  (params (OtherActor :type Actor%20Object%20Reference)))

(event EventTick
  (params (DeltaSeconds :type Float%20%28single-precision%29)))

(fn ConstructionScript)