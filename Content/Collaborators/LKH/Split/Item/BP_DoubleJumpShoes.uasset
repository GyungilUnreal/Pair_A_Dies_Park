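; Double jump shoes pickup that grants its ItemAbility to any actor overlapping its Box.
; On overlap it disables the Box collision and attaches itself to the foot_r socket through the ItemAbility component.
; It also spawns a BP_DoubleJumpShoe as the second shoe and attaches it to foot_l through that shoe's own ItemAbility.
; When the ability is consumed, it destroys the spawned left shoe.
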(event OnComponentBeginOverlap(Box)
  (params (OverlappedComponent :type Primitive%20Component%20Object%20Reference) (OtherActor :type Actor%20Object%20Reference) (OtherComp :type Primitive%20Component%20Object%20Reference) (OtherBodyIndex :type Integer) (bFromSweep :type Boolean) (SweepResult :type Hit%20Result%20Structure%20%28by%20ref%29))
  (Class|ItemAbilityComponent|GranttoActor (Variables|Default|GetItemAbility) OtherActor)
  (Collision|SetCollisionEnabled (Variables|Default|GetBox) "NoCollision")
  (Class|ItemAbilityComponent|AttachItemtoSocket (Variables|Default|GetItemAbility) OtherActor "foot_r")
  (bind _returnvalue (Game|SpawnActorfromClass "/Game/Collaborators/LKH/Split/Item/BP_DoubleJumpShoe.BP_DoubleJumpShoe_C" (Math|Transform|MakeTransform "0, 0, 0") "Undefined" "MultiplyWithRoot" 0 0))
  (Class|ItemAbilityComponent|AttachItemtoSocket (Variables|/Game/Collaborators/LKH/Split/Item/BP_DoubleJumpShoe.BP_DoubleJumpShoe_C|GetItemAbility _returnvalue) OtherActor "foot_l"))

(event OnAbilityConsumed(ItemAbility)
  (params (TargetActor :type Actor%20Object%20Reference))
  (Actor|DestroyActor (stale OnComponentBeginOverlap(Box) _returnvalue)))

(event EventBeginPlay)

(event Collision|EventActorBeginOverlap
  (params (OtherActor :type Actor%20Object%20Reference)))

(event EventTick
  (params (DeltaSeconds :type Float%20%28single-precision%29)))

(fn ConstructionScript)