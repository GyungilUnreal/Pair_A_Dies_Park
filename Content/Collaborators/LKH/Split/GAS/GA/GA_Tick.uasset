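; GA_Tick is a Gameplay Ability that appears to test per-tick waiting by staying active for about one second.
; On activation it stores and prints the game time, then calls the WaitTick event.
; WaitTick re-calls itself through Delay Until Next Tick to poll elapsed time each frame, then prints the time and ends the ability.
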(event Custom|WaitTick
  (if (>= (- (Utilities|Time|GetGameTimeinSeconds) (Variables|Default|GetStartTime)) 1.0)
    (Development|PrintString (Utilities|String|ToString(Float) (Utilities|Time|GetGameTimeinSeconds)))
    (Ability|EndAbility)
    (else
      (Utilities|FlowControl|DelayUntilNextTick)
      (CallFunction|WaitTick))))

(event Ability|EventActivateAbility
  (bind _output_get (Variables|Default|SetStartTime (Utilities|Time|GetGameTimeinSeconds)))
  (Development|PrintString (Utilities|String|ToString(Float) _output_get))
  (CallFunction|WaitTick))