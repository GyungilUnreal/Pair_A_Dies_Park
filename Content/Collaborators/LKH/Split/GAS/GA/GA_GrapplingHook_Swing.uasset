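; Gameplay ability that fires a grappling hook along the camera's aim and swings the avatar from it.
; Pressing input once hooked starts the swing, release ends it, and a five-second timeout or cancel also ends it, destroying the hook.
; A per-tick loop repositions the avatar using rope length, strips velocity away from the hook, adds tangential force and caps speed.
; Reel-in movement logic is present but unused.
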(event Custom|GetCurrentDistance
  (Variables|Default|SetCurDist (Math|Vector|Distance(Vector) (Transformation|GetActorLocation (Variables|Default|GetGrapplingHook)) (Transformation|GetActorLocation (Ability|GetAvatarActorfromActorInfo)))))

(event Custom|DoSwing
  (CallFunction|GetDir)
  (Transformation|SetActorLocation (Ability|GetAvatarActorfromActorInfo) (+ (Transformation|GetActorLocation (Variables|Default|GetGrapplingHook)) (* (Variables|Default|GetDir) (Variables|Default|GetRopeLength))) true false)
  (bind _as캐릭터 (Utilities|Casting|CastToCharacter (Ability|GetAvatarActorfromActorInfo)))
  (CallFunction|GetDir)
  (Variables|Default|SetCurVel (Variables|/Script/Engine.MovementComponent|GetVelocity (Variables|/Script/Engine.Character|GetCharacterMovement _as캐릭터)))
  (Variables|Default|SetAlong (Math|Vector|DotProduct (Variables|Default|GetCurVel) (Variables|Default|GetDir)))
  (if (< (Math|Vector|DotProduct (Variables|Default|GetCurVel) (Variables|Default|GetDir)) 0.0)
    (Variables|/Script/Engine.MovementComponent|SetVelocity (Variables|/Script/Engine.Character|GetCharacterMovement _as캐릭터) (- (Variables|Default|GetCurVel) (* (Variables|Default|GetDir) (Math|Vector|DotProduct (Variables|Default|GetCurVel) (Variables|Default|GetDir)))))
    (Physics|AddForce (Variables|/Script/Engine.Character|GetCharacterMovement _as캐릭터) (* (- (Variables|Default|GetCurVel) (* (Variables|Default|GetDir) (Variables|Default|GetAlong))) 5e+02))
    (bind _as캐릭터_2 (Utilities|Casting|CastToCharacter (Ability|GetAvatarActorfromActorInfo)))
    (Variables|/Script/Engine.MovementComponent|SetVelocity (Variables|/Script/Engine.Character|GetCharacterMovement _as캐릭터_2) (Math|Vector|VectorClampSizeMax (Variables|/Script/Engine.MovementComponent|GetVelocity (Variables|/Script/Engine.Character|GetCharacterMovement _as캐릭터_2)) 3e+03))))

(event Custom|WaitInputPress_ReelIn
  (bind _grapplinghook (Variables|Default|GetGrapplingHook))
  (bind _asynctaskproxy (Ability|Tasks|WaitInputPress false)
    (:then
      (Variables|Default|SetWaitInputTask _asynctaskproxy))
    (:OnPress
      (Utilities|IsValid _grapplinghook
        (:Is%20Valid
          (if (Variables|/Game/Collaborators/LKH/Split/Item/BP_GrapplingHook_Actor.BP_GrapplingHook_Actor_C|GetbIsHooked _grapplinghook)
            (GameplayTasks|EndTask (Variables|Default|GetAbilityEndTask))
            (CallFunction|WaitInputPressRelease)
            (CallFunction|WaitTick)
            (else
              (CallFunction|WaitInputPressReelin))))))))

(event Custom|WaitInputPress_Release
  (Ability|Tasks|WaitInputRelease false
    (:OnRelease
      (Ability|EndAbility))))

(event Custom|ReelInEnd
  (bind _as캐릭터 (Utilities|Casting|CastToCharacter (Ability|GetAvatarActorfromActorInfo)))
  (Variables|/Script/Engine.MovementComponent|SetVelocity (Variables|/Script/Engine.Character|GetCharacterMovement _as캐릭터) "0, 0, 0")
  (Transformation|SetActorLocation _as캐릭터 (Variables|Default|GetFixedLocation) false false))

(event Custom|WaitTick
  (CallFunction|DoSwing)
  (Utilities|FlowControl|DelayUntilNextTick)
  (CallFunction|WaitTick))

(event Custom|GetDir
  (Variables|Default|SetDir (Math|Vector|Normalize (- (Transformation|GetActorLocation (Variables|Default|GetGrapplingHook)) (Transformation|GetActorLocation (Ability|GetAvatarActorfromActorInfo))))))

(event Custom|ReelIn
  (bind _returnvalue (Ability|GetAvatarActorfromActorInfo))
  (bind _as캐릭터 (Utilities|Casting|CastToCharacter _returnvalue))
  (Physics|AddForce (Variables|/Script/Engine.Character|GetCharacterMovement _as캐릭터) (* (- (Transformation|GetActorLocation (Variables|Default|GetGrapplingHook)) (Transformation|GetActorLocation _returnvalue)) 1e+03)))

(event Ability|EventOnEndAbility
  (params (bWasCancelled :type Boolean))
  (bind _grapplinghook (Variables|Default|GetGrapplingHook))
  (Utilities|IsValid _grapplinghook
    (:Is%20Valid
      (Actor|DestroyActor _grapplinghook))))

(event Ability|EventActivateAbility
  (bind _returnvalue (Ability|GetAvatarActorfromActorInfo))
  (bind _returnvalue_2 (Game|SpawnActorfromClass "/Game/Collaborators/LKH/Split/Item/BP_GrapplingHook_Actor.BP_GrapplingHook_Actor_C" (Math|Transform|MakeTransform (Transformation|GetActorLocation _returnvalue) (Transformation|GetWorldRotation (Actor|GetComponentbyClass _returnvalue "/Script/Engine.CameraComponent"))) "Undefined" "MultiplyWithRoot" 0 0))
  (bind _output_get (Variables|Default|SetGrapplingHook _returnvalue_2))
  (Variables|/Game/Collaborators/LKH/Split/Item/BP_GrapplingHook_Actor.BP_GrapplingHook_Actor_C|SetShooter _output_get (Ability|GetAvatarActorfromActorInfo))
  (bind _asynctaskproxy (Ability|Tasks|WaitInputPress false)
    (:then
      (Variables|Default|SetWaitInputTask _asynctaskproxy)
      (bind _asynctaskproxy_2 (Ability|Tasks|WaitDelay 5.0)
        (:then
          (Variables|Default|SetAbilityEndTask _asynctaskproxy_2)
          (Ability|Tasks|WaitDelay 1.0
            (:OnFinish
              (|WaitCancel
                (:OnCancel
                  (Ability|EndAbility))))))
        (:OnFinish
          (Utilities|IsValid (Variables|Default|GetWaitInputTask)
            (:Is%20Valid
              (GameplayTasks|EndTask (Variables|Default|GetWaitInputTask)))
            (:Is%20Not%20Valid
              _))
          (Ability|EndAbility))))
    (:OnPress
      (Utilities|IsValid (Variables|Default|GetGrapplingHook)
        (:Is%20Valid
          (if (Variables|/Game/Collaborators/LKH/Split/Item/BP_GrapplingHook_Actor.BP_GrapplingHook_Actor_C|GetbIsHooked (Variables|Default|GetGrapplingHook))
            (GameplayTasks|EndTask (Variables|Default|GetAbilityEndTask))
            (CallFunction|WaitInputPressRelease)
            (CallFunction|WaitTick)
            (else
              (CallFunction|WaitInputPressReelin))))))))