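; Gameplay ability for a grappling hook that pulls the avatar without physics simulation.
; Activation spawns a hook actor ahead of the camera, hiding the non-authority copy, and ends after a timeout unless reeling starts.
; An input press once hooked starts a looping timer that accelerates CharacterMovement velocity toward the hook in Falling mode, up to a speed cap.
; Releasing input or a delayed-armed cancel ends the ability, which destroys the hook.
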(event Custom|WaitInputPress_ReelIn
  (bind _grapplinghook (Variables|Default|GetGrapplingHook))
  (bind _asynctaskproxy (Ability|Tasks|WaitInputPress false)
    (:then
      (Variables|Default|SetWaitInputTask _asynctaskproxy))
    (:OnPress
      (Utilities|IsValid _grapplinghook
        (:Is%20Valid
          (if (Variables|/Game/Collaborators/LKH/Split/Item/BP_GrapplingHook_Actor.BP_GrapplingHook_Actor_C|GetbIsHooked _grapplinghook)
            (GameplayTasks|EndTask (Variables|Default|GetAbilityEndTask))
            (CallFunction|WaitInputPressRelease)
            (CallFunction|WaitTick)
            (else
              (CallFunction|WaitInputPressReelin))))))))

(event Custom|WaitInputPress_Release
  (Ability|Tasks|WaitInputRelease false
    (:OnRelease
      (Ability|EndAbility))))

(event Custom|WaitTick
  (Utilities|Time|SetTimerbyEvent (delegate Custom|ReelIn) 0.01 true)
  (bind _as캐릭터 (Utilities|Casting|CastToCharacter (Ability|GetAvatarActorfromActorInfo)))
  (Pawn|Components|CharacterMovement|SetMovementMode (Variables|/Script/Engine.Character|GetCharacterMovement _as캐릭터) "MOVE_Falling" 0)
  (Utilities|FlowControl|Delay 0.5)
  (Pawn|Components|CharacterMovement|SetMovementMode (Variables|/Script/Engine.Character|GetCharacterMovement _as캐릭터) "MOVE_Falling" 0))

(event Custom|ReelIn
  (bind _returnvalue (Ability|GetAvatarActorfromActorInfo))
  (bind _grapplinghook (Variables|Default|GetGrapplingHook))
  (bind _returnvalue_2 (Transformation|GetActorLocation _grapplinghook))
  (bind _returnvalue_3 (Transformation|GetActorLocation _returnvalue))
  (bind _returnvalue_4 (- _returnvalue_2 _returnvalue_3))
  (bind _returnvalue_5 (Math|Vector|Normalize _returnvalue_4))
  (bind _returnvalue_6 (* _returnvalue_5 5e+03))
  (bind _as캐릭터 (Utilities|Casting|CastToCharacter _returnvalue))
  (if (> (Math|Vector|VectorLength (+ (* _returnvalue_5 5e+01) (Variables|/Script/Engine.MovementComponent|GetVelocity (Variables|/Script/Engine.Character|GetCharacterMovement _as캐릭터)))) (Math|Vector|VectorLength _returnvalue_6))
    (Variables|/Script/Engine.MovementComponent|SetVelocity (Variables|/Script/Engine.Character|GetCharacterMovement _as캐릭터) _returnvalue_6)
    (else
      (Variables|/Script/Engine.MovementComponent|SetVelocity (Variables|/Script/Engine.Character|GetCharacterMovement _as캐릭터) (+ (* _returnvalue_5 5e+01) (Variables|/Script/Engine.MovementComponent|GetVelocity (Variables|/Script/Engine.Character|GetCharacterMovement _as캐릭터)))))))

(event Ability|EventOnEndAbility
  (params (bWasCancelled :type Boolean))
  (bind _grapplinghook (Variables|Default|GetGrapplingHook))
  (Utilities|IsValid _grapplinghook
    (:Is%20Valid
      (Actor|DestroyActor _grapplinghook))))

(event Ability|EventActivateAbility
  (bind _returnvalue (Ability|GetAvatarActorfromActorInfo))
  (bind _returnvalue_2 (Actor|GetComponentbyClass _returnvalue "/Script/Engine.CameraComponent"))
  (bind _returnvalue_3 (Game|SpawnActorfromClass "/Game/Collaborators/LKH/Split/Item/BP_GrapplingHook_Actor.BP_GrapplingHook_Actor_C" (Math|Transform|MakeTransform (+ (Transformation|GetWorldLocation _returnvalue_2) (* (Math|Vector|GetForwardVector _returnvalue_2) 3e+02)) (Transformation|GetWorldRotation _returnvalue_2)) "Undefined" "MultiplyWithRoot" 0 0))
  (Ability|HasAuthority
    (:True
      _)
    (:False
      (Rendering|SetActorHiddenInGame _returnvalue_3 true)))
  (bind _output_get (Variables|Default|SetGrapplingHook _returnvalue_3))
  (Variables|/Game/Collaborators/LKH/Split/Item/BP_GrapplingHook_Actor.BP_GrapplingHook_Actor_C|SetShooter _output_get (Ability|GetAvatarActorfromActorInfo))
  (bind _asynctaskproxy (Ability|Tasks|WaitInputPress false)
    (:then
      (Variables|Default|SetWaitInputTask _asynctaskproxy)
      (bind _asynctaskproxy_2 (Ability|Tasks|WaitDelay 5.0)
        (:then
          (Variables|Default|SetAbilityEndTask _asynctaskproxy_2)
          (Ability|Tasks|WaitDelay 1.0
            (:OnFinish
              (|WaitCancel
                (:OnCancel
                  (Ability|EndAbility))))))
        (:OnFinish
          (Utilities|IsValid (Variables|Default|GetWaitInputTask)
            (:Is%20Valid
              (GameplayTasks|EndTask (Variables|Default|GetWaitInputTask)))
            (:Is%20Not%20Valid
              _))
          (Ability|EndAbility))))
    (:OnPress
      (Utilities|IsValid (Variables|Default|GetGrapplingHook)
        (:Is%20Valid
          (if (Variables|/Game/Collaborators/LKH/Split/Item/BP_GrapplingHook_Actor.BP_GrapplingHook_Actor_C|GetbIsHooked (Variables|Default|GetGrapplingHook))
            (GameplayTasks|EndTask (Variables|Default|GetAbilityEndTask))
            (CallFunction|WaitInputPressRelease)
            (CallFunction|WaitTick)
            (else
              (CallFunction|WaitInputPressReelin))))))))