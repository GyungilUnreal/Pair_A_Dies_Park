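; Gameplay ability that fires a grappling hook actor from the avatar along the camera's rotation and reels the character toward it.
; An input press re-arms until the hook has attached, then cancels the timeout and starts a per-tick loop adding force proportional to hook distance.
; Releasing input, the timeout, or a cancel after a short delay ends the ability, which destroys the hook.
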(event Custom|WaitInputPress_ReelIn
  (bind _grapplinghook (Variables|Default|GetGrapplingHook))
  (bind _asynctaskproxy (Ability|Tasks|WaitInputPress false)
    (:then
      (Variables|Default|SetWaitInputTask _asynctaskproxy))
    (:OnPress
      (Utilities|IsValid _grapplinghook
        (:Is%20Valid
          (if (Variables|/Game/Collaborators/LKH/Split/BP_GrapplingHook_Actor.BP_GrapplingHook_Actor_C|GetbIsHooked _grapplinghook)
            (GameplayTasks|EndTask (Variables|Default|GetAbilityEndTask))
            (CallFunction|WaitInputPressRelease)
            (CallFunction|WaitTick)
            (else
              (CallFunction|WaitInputPressReelin))))))))

(event Custom|WaitInputPress_Release
  (Ability|Tasks|WaitInputRelease false
    (:OnRelease
      (Ability|EndAbility))))

(event Custom|WaitTick
  (CallFunction|Reelin)
  (Utilities|FlowControl|DelayUntilNextTick)
  (CallFunction|WaitTick))

(event Custom|ReelIn
  (bind _returnvalue (Ability|GetAvatarActorfromActorInfo))
  (bind _as캐릭터 (Utilities|Casting|CastToCharacter _returnvalue))
  (Physics|AddForce (Variables|/Script/Engine.Character|GetCharacterMovement _as캐릭터) (* (- (Transformation|GetActorLocation (Variables|Default|GetGrapplingHook)) (Transformation|GetActorLocation _returnvalue)) 1e+03)))

(event Ability|EventOnEndAbility
  (params (bWasCancelled :type Boolean))
  (bind _grapplinghook (Variables|Default|GetGrapplingHook))
  (Utilities|IsValid _grapplinghook
    (:Is%20Valid
      (Actor|DestroyActor _grapplinghook))))

(event Ability|EventActivateAbility
  (bind _returnvalue (Ability|GetAvatarActorfromActorInfo))
  (bind _returnvalue_2 (Game|SpawnActorfromClass "/Game/Collaborators/LKH/Split/BP_GrapplingHook_Actor.BP_GrapplingHook_Actor_C" (Math|Transform|MakeTransform (Transformation|GetActorLocation _returnvalue) (Transformation|GetWorldRotation (Actor|GetComponentbyClass _returnvalue "/Script/Engine.CameraComponent"))) "Undefined" "MultiplyWithRoot" 0 0))
  (bind _output_get (Variables|Default|SetGrapplingHook _returnvalue_2))
  (Variables|/Game/Collaborators/LKH/Split/BP_GrapplingHook_Actor.BP_GrapplingHook_Actor_C|SetShooter _output_get (Ability|GetAvatarActorfromActorInfo))
  (bind _asynctaskproxy (Ability|Tasks|WaitInputPress false)
    (:then
      (Variables|Default|SetWaitInputTask _asynctaskproxy)
      (bind _asynctaskproxy_2 (Ability|Tasks|WaitDelay 5.0)
        (:then
          (Variables|Default|SetAbilityEndTask _asynctaskproxy_2)
          (Ability|Tasks|WaitDelay 1.0
            (:OnFinish
              (|WaitCancel
                (:OnCancel
                  (Ability|EndAbility))))))
        (:OnFinish
          (Utilities|IsValid (Variables|Default|GetWaitInputTask)
            (:Is%20Valid
              (GameplayTasks|EndTask (Variables|Default|GetWaitInputTask)))
            (:Is%20Not%20Valid
              _))
          (Ability|EndAbility))))
    (:OnPress
      (Utilities|IsValid (Variables|Default|GetGrapplingHook)
        (:Is%20Valid
          (if (Variables|/Game/Collaborators/LKH/Split/BP_GrapplingHook_Actor.BP_GrapplingHook_Actor_C|GetbIsHooked (Variables|Default|GetGrapplingHook))
            (GameplayTasks|EndTask (Variables|Default|GetAbilityEndTask))
            (CallFunction|WaitInputPressRelease)
            (CallFunction|WaitTick)
            (else
              (CallFunction|WaitInputPressReelin))))))))