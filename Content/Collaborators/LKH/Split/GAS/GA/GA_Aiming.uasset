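; GA_Aiming is a Gameplay Ability that puts BP_Split_Character into aim mode until the input is released.
; On activation it shows a crosshair widget for the locally controlled player and lerps the CameraBoom socket offset to the aiming position over about a third of a second.
; The lerp is a self-calling next-tick loop timed from game seconds.
; Ending the ability snaps the offset back to zero and removes the crosshair.
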(event Custom|WaitTick
  (if (not (>= (Variables|Default|GetDeltaTime) 0.33))
    (CallFunction|MoveCameraOffset)
    (Utilities|FlowControl|DelayUntilNextTick)
    (CallFunction|WaitTick)))

(event Custom|MoveCameraOffset
  (bind _returnvalue (Utilities|Time|GetTimeSeconds))
  (bind _starttime (Variables|Default|GetStartTime))
  (bind _returnvalue_2 (- _returnvalue _starttime))
  (Variables|Default|SetDeltaTime _returnvalue_2)
  (Variables|/Script/Engine.SpringArmComponent|SetSocketOffset (Variables|Default|GetCamera%20Boom) (Math|Vector|Lerp(Vector) (Variables|Default|GetStartLoc) (Variables|Default|GetAimingLoc) (* _returnvalue_2 3.0))))

(event Custom|PreTick
  (Variables|Default|SetStartTime (Utilities|Time|GetTimeSeconds))
  (Pawn|IsLocallyControlled
    (:True
      (bind _returnvalue (UserInterface|CreateWidget "/Game/Collaborators/LKH/Split/WBP_Crosshair.WBP_Crosshair_C"))
      (UserInterface|Viewport|AddtoPlayerScreen _returnvalue))))

(event Ability|EventActivateAbility
  (bind _asbp_split_character (Utilities|Casting|CastToBP_Split_Character (Ability|GetAvatarActorfromActorInfo)))
  (Variables|Default|SetCamera%20Boom (Variables|/Script/Pair_A_Dies_Park.Split_Character|GetCameraBoom _asbp_split_character))
  (Ability|Tasks|WaitInputRelease false
    (:then
      (CallFunction|PreTick)
      (CallFunction|WaitTick))
    (:OnRelease
      (Ability|EndAbility))))

(event Ability|EventOnEndAbility
  (params (bWasCancelled :type Boolean))
  (Variables|/Script/Engine.SpringArmComponent|SetSocketOffset (Variables|Default|GetCamera%20Boom) "0, 0, 0")
  (Pawn|IsLocallyControlled
    (:True
      (Widget|RemovefromParent (stale Custom|PreTick _returnvalue)))))