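; Gameplay Ability that gives the avatar Character a mid-air second jump, with an item component as its source.
; It ends immediately if a normal jump is possible, otherwise it temporarily raises JumpMaxCount and retries.
; A successful retry commits, jumps, fires the DoubleJump gameplay cue and ends after a short delay, restoring the single-jump limit.
; Committing notifies the source ItemAbilityComponent that the ability was consumed.
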(event Ability|EventActivateAbility
  (bind _as캐릭터 (Utilities|Casting|CastToCharacter (Ability|GetAvatarActorfromActorInfo)))
  (if (Character|CanJump _as캐릭터)
    (Ability|EndAbility)
    (else
      (Variables|/Script/Engine.Character|SetJumpMaxCount _as캐릭터 2)
      (if (Character|CanJump _as캐릭터)
        (Ability|CommitAbility)
        (Character|Jump _as캐릭터)
        (GameplayCue|ExecuteGameplayCue :GameplayCueTag "(TagName=\"GameplayCue.Ability.DoubleJump\")")
        (Utilities|FlowControl|Delay 0.2)
        (Ability|EndAbility)
        (else
          (Ability|EndAbility))))))

(event Ability|EventOnEndAbility
  (params (bWasCancelled :type Boolean))
  (bind _as캐릭터 (Utilities|Casting|CastToCharacter (Ability|GetAvatarActorfromActorInfo)))
  (Variables|/Script/Engine.Character|SetJumpMaxCount _as캐릭터 1))

(event Ability|EventCommitExecute
  (bind _asitem_ability_component (Utilities|Casting|CastToItemAbilityComponent (Ability|GetCurrentSourceObject)))
  (Class|ItemAbilityComponent|NotifyAbilityConsumed _asitem_ability_component (Ability|GetOwningActorfromActorInfo)))